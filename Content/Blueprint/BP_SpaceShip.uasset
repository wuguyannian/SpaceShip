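; BP_SpaceShip is a spaceship actor with a spawn animation, movement, health and explosive death.
; A timeline lerps it by a spawn offset and rotation, then enables per-tick swept movement by GetCurrentSpeed, which returns zero here, apparently for child classes to override.
; Damage lowers clamped health, and Heal reuses that path with negative damage.
; At zero health it plays explosion effects, disables collision and expires almost immediately.
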(event `self.ReceiveBeginPlay`
  (bind (_returnvalue_roll _returnvalue_pitch _returnvalue_yaw) (`KismetMathLibrary.BreakRotator` (`self.K2_GetActorRotation`)))
  (bind _initiallocation (`self.InitialLocation`))
  ;[1 1 1] 初始动画
  (set `self.InitialLocation` (`self.K2_GetActorLocation`))
  (set `self.InitialYaw` _returnvalue_yaw)
  (bind (_direction _movement_lerp) (`Timeline|SpawnAnimation`)
    (:`Update`
      (`self.K2_SetActorLocation` (`KismetMathLibrary.VLerp` _initiallocation (+ _initiallocation (`self.SpawnOffset`)) _movement_lerp))
      (`self.K2_SetActorRotation` (`KismetMathLibrary.RLerp` (struct) (`KismetMathLibrary.MakeRotator` 0.0 0.0 (+ (`self.InitialYaw`) (`self.SpawnRotation`))) _movement_lerp)))
    (:`Finished`
      (set `self.MovementEnabled` true))))

(event `self.ReceiveTick`
  (params (DeltaSeconds :type "Float (single-precision)"))
  ;[1 1 1] 移动
  (if (`self.MovementEnabled`)
    (`self.K2_SetActorLocation` (+ (`self.K2_GetActorLocation`) (`self.GetCurrentSpeed` DeltaSeconds)) true)))

(event `self.ReceiveAnyDamage`
  (params (Damage :type "Float (single-precision)") (DamageType :type "DamageType Object Reference") (InstigatedBy :type "Controller Object Reference") (DamageCauser :type "Actor Object Reference"))
  ;[1 1 1] 伤害处理
  (bind _output_get (set `self.Health` (`KismetMathLibrary.FClamp` (- (`self.Health`) Damage) 0.0 (`self.HealthMax`))))
  (if (<= _output_get 0.0)
    (`self.OnDeath`)))

(event `OnDeath`
  (bind _returnvalue (`self.K2_GetActorLocation`))
  ;[1 1 1] 死亡
  (`GameplayStatics.PlaySoundAtLocation` "/Game/Audio/SCue_Explode.SCue_Explode" _returnvalue (struct) 1.0 1.0 0.0 null null null)
  (`GameplayStatics.SpawnEmitterAtLocation` (`self.ExplosionType`) _returnvalue)
  (`PrimitiveComponent.SetCollisionEnabled` (`self.SpaceShip`) "NoCollision")
  (`self.SetLifeSpan` 0.01))

(fn `GetCurrentSpeed`
  (params (Delta :type "Float (double-precision)"))
  (returns (Speed :type "Vector Structure"))
  (return (0.0 0.0 0.0)))

(fn `Heal`
  (params (Heal :type "Float (double-precision)"))
  (`GameplayStatics.ApplyDamage` self (* Heal -1.0) null self))

(fn `UserConstructionScript`
  (set `self.Health` (`self.HealthMax`)))