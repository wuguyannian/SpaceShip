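; Player spaceship Blueprint that moves sideways and fires bullets.
; GetCurrentSpeed eases the speed toward MoveRight input and returns it as a Y-only vector, while Tick smoothly yaws the ship in proportion to that speed.
; Pressing Fire shoots immediately and starts a looping timer until release, each shot spawning a colored BP_Bullet with upward Z speed and playing a sound.
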(event `self.ReceiveBeginPlay`
  (`parent.ReceiveBeginPlay`))

(event `self.ReceiveTick`
  (params (DeltaSeconds :type "Float (single-precision)"))
  ;[1 1 1] 移动效果
  (`parent.ReceiveTick` DeltaSeconds)
  (`self.K2_SetActorRotation` (`KismetMathLibrary.RInterpTo` (`self.K2_GetActorRotation`) (`KismetMathLibrary.MakeRotator` 0.0 0.0 (+ (* (`self.CurrentSpeed`) -15.0) (`self.InitialYaw`))) DeltaSeconds 20.0)))

(event `OnFire`
  (`|SpawnActorFromClass` "/Game/Blueprint/BP_Bullet.BP_Bullet_C" (`self.GetTransform`) "AdjustIfPossibleButDontSpawnIfColliding" "OverrideRootScale" null self (make `LinearColor` 2.0 0.5 1.0 1.0) (0.0 0.0 700.0) null :!label _label)
  (`GameplayStatics.PlaySoundAtLocation` "/Game/Audio/SCue_Fire.SCue_Fire" (`self.K2_GetActorLocation`) (struct) 1.0 1.0 0.0 null null null))

(event `InputAction|Fire`
  (params (Key :type "Key Structure"))
  (:`Pressed`
    (`KismetSystemLibrary.K2_SetTimer` null "OnFire" 0.2 true)
    (goto _label))
  (:`Released`
    (`KismetSystemLibrary.K2_ClearTimer` null "OnFire")))

(fn `GetCurrentSpeed`
  (params (Delta :type "Float (double-precision)"))
  (returns (Speed :type "Vector Structure"))
  (bind _output_get (set `self.CurrentSpeed` (`KismetMathLibrary.FInterpTo` (`self.CurrentSpeed`) (* Delta (`self.GetInputAxisValue`) (`self.MovementSpeed`)) Delta 4.0)))
  (return (`KismetMathLibrary.MakeVector` 0.0 _output_get)))

(fn `UserConstructionScript`
  (`parent.UserConstructionScript`))