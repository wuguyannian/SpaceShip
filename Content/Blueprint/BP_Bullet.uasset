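; BP_Bullet is a colored projectile actor that damages what it hits.
; It moves by a local offset each tick without sweeping, tinting a dynamic material and light with its bullet color on BeginPlay.
; On overlap with any actor other than its owner, it applies fixed damage, spawns a pixel explosion and destroys itself.
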(event `self.ReceiveBeginPlay`
  (bind _bulletcolor (`self.BulletColor`))
  ;[1 1 1] 初始
  (`MaterialInstanceDynamic.SetVectorParameterValue` (`self.BulletMaterial`) "Color2" _bulletcolor)
  (`LightComponent.SetLightColor` (`self.Light`) _bulletcolor true))

(event `self.ReceiveTick`
  (params (DeltaSeconds :type "Float (single-precision)"))
  ;[1 1 1] 移动
  (`self.K2_AddActorLocalOffset` (* (`self.Speed`) DeltaSeconds)))

(event `self.Bullet.OnComponentBeginOverlap`
  (params (OverlappedComponent :type "PrimitiveComponent Object Reference") (OtherActor :type "Actor Object Reference") (OtherComp :type "PrimitiveComponent Object Reference") (OtherBodyIndex :type Integer) (bFromSweep :type Boolean) (SweepResult :type "HitResult Structure (by ref)"))
  ;[1 1 1] 撞击
  (if (!= (`self.BulletOwner`) OtherActor)
    (`GameplayStatics.ApplyDamage` OtherActor 20.0)
    (`self.OnDeath`)))

(event `OnDeath`
  ;[1 1 1] 死亡
  (`GameplayStatics.SpawnEmitterAtLocation` "/Game/Art/Particles/P_Pixel_Explosion.P_Pixel_Explosion" (`self.K2_GetActorLocation`))
  (`self.K2_DestroyActor`))

(fn `UserConstructionScript`
  (bind _returnvalue (`PrimitiveComponent.CreateDynamicMaterialInstance` (`self.Bullet`) 0 null "None"))
  (set `self.BulletMaterial` _returnvalue))