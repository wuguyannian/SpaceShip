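; Enemy spaceship that moves sideways while drifting vertically and fires colored bullets at the player.
; Tick uses a random Delay to pace OnFire, which shoots only when the player is roughly aligned on the X axis.
; Hitting a pawn damages it and triggers death, while other hits flip the sideways direction used by GetCurrentSpeed.
; The parent class supplies base behavior, and SyncHP updates the health widget on spawn and damage.
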(event `OnFire`
  (bind _returnvalue (`GameplayStatics.GetPlayerPawn` 0))
  ;[1 1 1] 射击
  (`/Engine/EditorBlueprintResources/StandardMacros.IsValid` _returnvalue
    (:`Is Valid`
      (if (<= (`KismetMathLibrary.VSize` (* (- (`self.K2_GetActorLocation` _returnvalue) (`self.K2_GetActorLocation`)) (1.0 0.0 0.0))) 120.0)
        (`|SpawnActorFromClass` "/Game/Blueprint/BP_Bullet.BP_Bullet_C" (`self.GetTransform`) "AdjustIfPossibleButDontSpawnIfColliding" "OverrideRootScale" null self (make `LinearColor` 1.0 0.3 0.05 1.0) (0.0 0.0 -200.0) null)
        (`GameplayStatics.PlaySoundAtLocation` "/Game/Audio/SCue_Fire.SCue_Fire" (`self.K2_GetActorLocation`) (struct) 1.0 1.0 0.0 null null null)))))

(event `self.ReceiveTick`
  (params (DeltaSeconds :type "Float (single-precision)"))
  ;[1 1 1] 攻击
  (`parent.ReceiveTick` DeltaSeconds)
  (`/Engine/EditorBlueprintResources/StandardMacros.IsValid` (`GameplayStatics.GetPlayerPawn` 0)
    (:`Is Valid`
      (`KismetSystemLibrary.Delay` (`KismetMathLibrary.RandomFloatInRange` 0.4 0.8))
      (`self.OnFire`))))

(event `self.ReceiveHit`
  (params (MyComp :type "PrimitiveComponent Object Reference") (Other :type "Actor Object Reference") (OtherComp :type "PrimitiveComponent Object Reference") (bSelfMoved :type Boolean) (HitLocation :type "Vector Structure") (HitNormal :type "Vector Structure") (NormalImpulse :type "Vector Structure") (Hit :type "HitResult Structure (by ref)"))
  ;[1 1 1] 撞击
  (cast `Pawn` Other
    (:`then`
      (`GameplayStatics.ApplyDamage` Other 90.0)
      (`self.OnDeath`))
    (:`CastFailed`
      (set `self.MoveDirection` (not (`self.MoveDirection`))))))

(event `self.ReceiveAnyDamage`
  (params (Damage :type "Float (single-precision)") (DamageType :type "DamageType Object Reference") (InstigatedBy :type "Controller Object Reference") (DamageCauser :type "Actor Object Reference"))
  ;[1 1 1] 同步血量
  (`parent.ReceiveAnyDamage` Damage null null null)
  (`self.SyncHP`))

(event `self.ReceiveBeginPlay`
  ;[1 1 1] 同步血量
  (`parent.ReceiveBeginPlay`)
  (`self.SyncHP`))

(fn `GetCurrentSpeed`
  (params (Delta :type "Float (double-precision)"))
  (returns (Speed :type "Vector Structure"))
  (return (`KismetMathLibrary.MakeVector` 0.0 (* (`KismetMathLibrary.SelectFloat` 1.0 -1.0 (`self.MoveDirection`)) (`self.MovementSpeed`) Delta) (* Delta (`self.MovementSpeedDown`)))))

(fn `SyncHP`
  (bind _widget (`self.Widget`))
  (`/Engine/EditorBlueprintResources/StandardMacros.IsValid` _widget
    (:`Is Valid`
      (bind _aswb_health_enemy (cast `/Game/Art/UI/WB_HealthEnemy` (`WidgetComponent.GetUserWidgetObject` _widget)))
      (`/Game/Art/UI/WB_HealthEnemy.SetHealth` _aswb_health_enemy (`KismetMathLibrary.FTrunc` (`self.Health`)) (`KismetMathLibrary.FTrunc` (`self.HealthMax`))))))

(fn `UserConstructionScript`
  (`parent.UserConstructionScript`))