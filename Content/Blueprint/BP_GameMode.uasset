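; Game mode for a spaceship shooter that runs the match: HUD, player lives and health, score, enemy spawning, pickups and game over.
; InitGame spawns the player at a tagged actor and starts a self-recalling timed loop spawning enemies at random horizontal offsets.
; Bound destroy, damage and pickup events drive respawns, score, random item drops and HUD updates.
; StartGame, Replay and GotoMainMenu handle level flow, the latter two with camera fades.
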(event `self.ReceiveBeginPlay`
  ;[1 1 1] 初始
  (`GameplayStatics.PlaySoundAtLocation` "/Game/Audio/BackGround.BackGround" (0.0 0.0 0.0) (struct) 1.0 1.0 0.0 null null null))

(event `SpawnPlayer`
  ;[1 1 1] 创建玩家
  (bind _outactors (`GameplayStatics.GetAllActorsWithTag` "Player"))
  (bind _returnvalue (`|SpawnActorFromClass` "/Game/Blueprint/BP_SpaceShipPlayer.BP_SpaceShipPlayer_C" (`self.GetTransform` (`|GetArrayItem` _outactors)) "AlwaysSpawn" "OverrideRootScale" null null))
  (`Controller.Possess` (`GameplayStatics.GetPlayerController` 0) _returnvalue)
  ;[1 1 1] 死亡处理
  (add `self.OnDestroyed` _returnvalue (delegate `OnPlayerKilled`))
  ;[1 1 1] 血量处理
  (add `self.OnTakeAnyDamage` _returnvalue (delegate `OnPlayerTakeDamage`))
  (`/Game/Art/UI/WB_GameStatus.SetPlayerHealth` (`self.GameStatus`) 1.0))

(event `OnPlayerTakeDamage` :!signature `self.OnTakeAnyDamage`
  (params (DamagedActor :type "Actor Object Reference") (Damage :type "Float (double-precision)") (DamageType :type "DamageType Object Reference") (InstigatedBy :type "Controller Object Reference") (DamageCauser :type "Actor Object Reference"))
  ;[1 1 1] 血量处理
  (bind _asbp_space_ship (cast `/Game/Blueprint/BP_SpaceShip` DamagedActor))
  (`/Game/Art/UI/WB_GameStatus.SetPlayerHealth` (`self.GameStatus`) (/ (`/Game/Blueprint/BP_SpaceShip.Health` _asbp_space_ship) (`/Game/Blueprint/BP_SpaceShip.HealthMax` _asbp_space_ship))))

(event `OnPlayerKilled` :!signature `self.OnDestroyed`
  (params (DestroyedActor :type "Actor Object Reference"))
  ;[1 1 1] 死亡处理
  (clear `self.OnTakeAnyDamage` DestroyedActor)
  (set `self.EnemySpawnning` false)
  (`self.OnShipDestroyed` DestroyedActor)
  (`self.ModifyLife` -1)
  (if (> (`self.Life`) 0)
    (`KismetSystemLibrary.Delay` 3.0)
    (`self.SpawnPlayer`)
    (set `self.EnemySpawnning` true)
    (else
      (`KismetSystemLibrary.Delay` 1.0)
      (`self.GameOver`))))

(event `SpawnEnemy`
  (bind _enemyspawnhorizontalrange (`self.EnemySpawnHorizontalRange`))
  ;[1 1 1] 创建敌人
  (if (`self.EnemySpawnning`)
    (bind _outactors (`GameplayStatics.GetAllActorsWithTag` "Enemy"))
    (bind _returnvalue (`|SpawnActorFromClass` "/Game/Blueprint/BP_SpaceShipEnemy.BP_SpaceShipEnemy_C" (`KismetMathLibrary.ComposeTransforms` (`self.GetTransform` (`|GetArrayItem` _outactors)) (`KismetMathLibrary.MakeTransform` (`KismetMathLibrary.MakeVector` 0.0 (`KismetMathLibrary.RandomFloatInRange` (* _enemyspawnhorizontalrange -1.0) _enemyspawnhorizontalrange)))) "AlwaysSpawn" "OverrideRootScale" null null))
    ;[1 1 1] 死亡处理
    (add `self.OnDestroyed` _returnvalue (delegate `OnEnemyKilled`))))

(event `OnEnemyKilled` :!signature `self.OnDestroyed`
  (params (DestroyedActor :type "Actor Object Reference"))
  ;[1 1 1] 死亡处理
  (`self.ProcessItemDrop` DestroyedActor)
  (`self.AddScore` DestroyedActor)
  (`self.OnShipDestroyed` DestroyedActor))

(event `StartSpawnEnemy`
  ;[1 1 1] 敌人波次
  (`self.SpawnEnemy`)
  (`KismetSystemLibrary.Delay` (`KismetMathLibrary.RandomFloatInRange` 5.0 5.0))
  (`self.StartSpawnEnemy`))

(event `InitUI`
  ;[1 1 1] 创建界面
  (bind _returnvalue (`|CreateWidget` "/Game/Art/UI/WB_GameStatus.WB_GameStatus_C"))
  (bind _output_get (set `self.GameStatus` _returnvalue))
  (`UserWidget.AddToViewport` _output_get 0)
  (set `PlayerController.bShowMouseCursor` false (`GameplayStatics.GetPlayerController` 0)))

(event `InitGame`
  ;[1 1 1] 初始游戏
  (`self.InitUI`)
  (`self.SpawnPlayer`)
  (`self.StartSpawnEnemy`)
  (`self.SyncScore`)
  (`self.SyncLife`))

(event `DropItem`
  (params (Instigator :type "Actor Object Reference") (Index :type Integer))
  ;[1 1 1] 掉落处理
  (bind _returnvalue (`|SpawnActorFromClass` "/Game/Blueprint/BP_Item.BP_Item_C" (`self.GetTransform` Instigator) "AlwaysSpawn" "OverrideRootScale" null (`|GetArrayItem` (`self.DrapList`) Index) null))
  (add `/Game/Blueprint/BP_Item.OnPickup` _returnvalue (delegate `OnPickup`)))

(event `OnPickup`
  (params (Instigator :type "Actor Object Reference") (ItemType :type "/Game/Blueprint/E_ItemType Enum" :default "NewEnumerator0"))
  ;[1 1 1] 掉落处理
  (bind _asbp_space_ship_player (cast `/Game/Blueprint/BP_SpaceShipPlayer` Instigator))
  (switch `/Game/Blueprint/E_ItemType` ItemType
    (:`NewEnumerator0`
      (`self.ModifyLife` 1)
      (`GameplayStatics.PlaySound2D` "/Game/Audio/SCue_Life.SCue_Life" 1.0 1.0 0.0 null null))
    (:`NewEnumerator1`
      (`/Game/Blueprint/BP_SpaceShip.Heal` _asbp_space_ship_player 15.0)
      (`GameplayStatics.PlaySound2D` "/Game/Audio/SCue_Health.SCue_Health" 1.0 1.0 0.0 null null))))

(event `ProcessItemDrop`
  (params (Instigator :type "Actor Object Reference"))
  (bind _returnvalue (`KismetMathLibrary.RandomInteger` 100))
  ;[1 1 1] 掉落处理
  (if (<= _returnvalue 5)
    (`self.DropItem` Instigator)
    (elif (<= _returnvalue 15)
      (`self.DropItem` Instigator 1))))

(event `GameOver`
  (bind _returnvalue (`GameplayStatics.GetPlayerController` 0))
  ;[1 1 1] 游戏结束
  (bind _returnvalue_2 (`|CreateWidget` "/Game/Art/UI/WB_GameFinish.WB_GameFinish_C"))
  (`/Game/Art/UI/WB_GameFinish.SetScore` _returnvalue_2 (`self.Score`))
  (`UserWidget.AddToViewport` _returnvalue_2 0)
  (`GameplayStatics.SetGamePaused` true)
  (`WidgetBlueprintLibrary.SetInputMode_GameAndUIEx` _returnvalue _returnvalue_2 "LockAlways")
  (set `PlayerController.bShowMouseCursor` true _returnvalue))

(event `StartGame`
  ;[1 1 1] 开始游戏
  (bind _outactors (`GameplayStatics.GetAllActorsOfClass` "/Script/LevelSequence.LevelSequenceActor"))
  (bind _output (`|GetArrayItem` _outactors))
  (`/Engine/EditorBlueprintResources/StandardMacros.IsValid` _output
    (:`Is Valid`
      (`MovieSceneSequencePlayer.Play` (`LevelSequenceActor.SequencePlayer` _output)))
    (:`Is Not Valid`
      (`GameplayStatics.OpenLevel` "GameLevel"))))

(event `Replay`
  ;[1 1 1] 重新开始
  (`WidgetLayoutLibrary.RemoveAllWidgets`)
  (`self.SceneFadeout` 0.5)
  (`GameplayStatics.SetGamePaused` false)
  (`KismetSystemLibrary.Delay` 0.5)
  (`GameplayStatics.OpenLevel` "GameLevel"))

(event `GotoMainMenu`
  (`WidgetLayoutLibrary.RemoveAllWidgets`)
  (`self.SceneFadeout` 0.5)
  (`GameplayStatics.SetGamePaused` false)
  (`KismetSystemLibrary.Delay` 0.35)
  (`GameplayStatics.OpenLevel` "MainMenu"))

(fn `AddScore`
  (params (Instigator :type "Actor Object Reference"))
  (bind _asbp_space_ship_enemy (cast `/Game/Blueprint/BP_SpaceShipEnemy` Instigator))
  (set `self.Score` (+ (`self.Score`) (`/Game/Blueprint/BP_SpaceShipEnemy.Score` _asbp_space_ship_enemy)))
  (`self.SyncScore`))

(fn `ModifyLife`
  (params (Value :type Integer))
  (set `self.Life` (`KismetMathLibrary.Clamp` (+ Value (`self.Life`)) 0 9999))
  (`self.SyncLife`))

(fn `SceneFadeout`
  (params (duration :type "Float (double-precision)"))
  (`PlayerCameraManager.StartCameraFade` (`PlayerController.PlayerCameraManager` (`GameplayStatics.GetPlayerController` 0)) 0.0 1.0 duration (struct :`A` 1.0) true true))

(fn `SyncLife`
  (`/Game/Art/UI/WB_GameStatus.SetPlayerLife` (`self.GameStatus`) (`self.Life`)))

(fn `SyncScore`
  (`/Game/Art/UI/WB_GameStatus.SetPlayerScore` (`self.GameStatus`) (`self.Score`)))

(fn `UserConstructionScript`)