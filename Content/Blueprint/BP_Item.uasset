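; BP_Item is a moving pickup that reports its item type to whatever overlaps it.
; The construction script creates a dynamic material on the mesh, and BeginPlay tints it with the color from ItemInfo.
; Tick shifts it by Speed in local space without sweeping.
; On overlap it disables mesh collision, fires the OnPickup dispatcher with the overlapping actor and item type, then destroys itself.
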(event `self.ReceiveBeginPlay`
  (bind (_iteminfo_itemtype _iteminfo_itemcolor) (break `/Game/Blueprint/S_DropItem` (`self.ItemInfo`)))
  (`MaterialInstanceDynamic.SetVectorParameterValue` (`self.Material`) "Color" _iteminfo_itemcolor))

(event `self.ReceiveTick`
  (params (DeltaSeconds :type "Float (single-precision)"))
  ;[1 1 1] 移动
  (`self.K2_AddActorLocalOffset` (* (`self.Speed`) DeltaSeconds)))

(event `self.StaticMesh.OnComponentBeginOverlap`
  (params (OverlappedComponent :type "PrimitiveComponent Object Reference") (OtherActor :type "Actor Object Reference") (OtherComp :type "PrimitiveComponent Object Reference") (OtherBodyIndex :type Integer) (bFromSweep :type Boolean) (SweepResult :type "HitResult Structure (by ref)"))
  (bind _iteminfo_itemtype (break `/Game/Blueprint/S_DropItem` (`self.ItemInfo`)))
  ;[1 1 1] 处理拾取
  (`PrimitiveComponent.SetCollisionEnabled` (`self.StaticMesh`) "NoCollision")
  (`self.OnPickup` OtherActor _iteminfo_itemtype)
  (`self.K2_DestroyActor`))

(fn `UserConstructionScript`
  (bind _returnvalue (`PrimitiveComponent.CreateDynamicMaterialInstance` (`self.StaticMesh`) 0 null "None"))
  (set `self.Material` _returnvalue))